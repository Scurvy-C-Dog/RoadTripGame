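; BP_Player is the player pawn, which can board vehicles it overlaps.
; It adds the IMC_Player Enhanced Input mapping context on possession and removes it when unpossessed.
; On IA_Interact, it loops over overlapping BP_Vehicle_Base actors and has player controller 0 possess them, then hides itself and disables capsule and mesh collision.
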(event Input|EnhancedActionEvents|EnhancedInputActionIA_Interact
  (params (ActionValue :type Boolean) (ElapsedSeconds :type Float%20%28double-precision%29) (TriggeredSeconds :type Float%20%28double-precision%29) (InputAction :type Input%20Action%20Object%20Reference :default "/Game/Player/Input/Actions/IA_Interact.IA_Interact"))
  (:Triggered
    (for _array_element (Collision|GetOverlappingActors "/Game/Player/BP_Vehicle_Base.BP_Vehicle_Base_C" :!class /Script/Engine.Actor)
      (bind _asbp_vehicle_base (Utilities|Casting|CastToBP_Vehicle_Base _array_element))
      (Pawn|Possess (Game|GetPlayerController 0) _asbp_vehicle_base)
      (Rendering|SetActorHiddenInGame true)
      (Collision|SetCollisionEnabled (Variables|Default|GetCapsuleComponent) "NoCollision"))))

(event EventPossessed
  (params (NewController :type Controller%20Object%20Reference))
  (Input|AddMappingContext (PlayerController|LocalPlayerSubsystems|GetEnhancedInputLocalPlayerSubsystem (Game|GetPlayerController 0)) "/Game/Player/Input/IMC_Player.IMC_Player" 0 "(bIgnoreAllPressedKeysUntilRelease=True,bForceImmediately=False,bNotifyUserSettings=False)"))

(event EventUnpossessed
  (params (OldController :type Controller%20Object%20Reference))
  (Input|RemoveMappingContext (PlayerController|LocalPlayerSubsystems|GetEnhancedInputLocalPlayerSubsystem (Game|GetPlayerController 0)) "/Game/Player/Input/IMC_Player.IMC_Player" "(bIgnoreAllPressedKeysUntilRelease=True,bForceImmediately=False,bNotifyUserSettings=False)"))

(fn ConstructionScript
  (|CallParentFunction))