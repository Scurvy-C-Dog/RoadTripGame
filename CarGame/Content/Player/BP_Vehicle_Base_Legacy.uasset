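; Legacy base Blueprint for a drivable player vehicle that swaps the IMC_Car Enhanced Input context on possess and unpossess.
; Input actions feed throttle, steering, brake and handbrake to the vehicle movement component, while look input yaws a spring arm that eases back to center each tick.
; Tick also adds angular damping while airborne to steady the car.
; Exit teleports the hidden BP_Player to an arrow, restores its visibility and collision, and possesses it.
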(event Custom|InterpsToOriginalRotation
  (bind _springarm (Variables|Default|GetSpringArm))
  (Transformation|SetRelativeRotation _springarm (Math|Rotator|MakeRotator 0.0 0.0 (Math|Interpolation|FInterpTo (.yaw (Variables|/Script/Engine.SceneComponent|GetRelativeRotation _springarm)) 0.0 (Utilities|Time|GetWorldDeltaSeconds) 1.0)) false false))

(event Input|EnhancedActionEvents|EnhancedInputActionIA_Throttle
  (params (ActionValue :type Float%20%28double-precision%29) (ElapsedSeconds :type Float%20%28double-precision%29) (TriggeredSeconds :type Float%20%28double-precision%29) (InputAction :type Input%20Action%20Object%20Reference :default "/Game/Player/Input/Actions/IA_Throttle.IA_Throttle"))
  (:Triggered
    (Class|ChaosVehicleMovementComponent|SetThrottleInput (Variables|Default|GetVehicle%20Movement%20Component) ActionValue :!label _label))
  (:Completed
    (goto _label)))

(event Input|EnhancedActionEvents|EnhancedInputActionIA_Steering
  (params (ActionValue :type Float%20%28double-precision%29) (ElapsedSeconds :type Float%20%28double-precision%29) (TriggeredSeconds :type Float%20%28double-precision%29) (InputAction :type Input%20Action%20Object%20Reference :default "/Game/Player/Input/Actions/IA_Steering.IA_Steering"))
  (:Triggered
    (Class|ChaosVehicleMovementComponent|SetSteeringInput (Variables|Default|GetVehicle%20Movement%20Component) ActionValue :!label _label))
  (:Completed
    (goto _label)))

(event Input|EnhancedActionEvents|EnhancedInputActionIA_Break
  (params (ActionValue :type Float%20%28double-precision%29) (ElapsedSeconds :type Float%20%28double-precision%29) (TriggeredSeconds :type Float%20%28double-precision%29) (InputAction :type Input%20Action%20Object%20Reference :default "/Game/Player/Input/Actions/IA_Break.IA_Break"))
  (:Triggered
    (Class|ChaosVehicleMovementComponent|SetBrakeInput (Variables|Default|GetVehicle%20Movement%20Component) ActionValue))
  (:Completed
    (Class|ChaosVehicleMovementComponent|SetBrakeInput (Variables|Default|GetVehicle%20Movement%20Component) ActionValue)))

(event Input|EnhancedActionEvents|EnhancedInputActionIA_Handbreak
  (params (ActionValue :type Boolean) (ElapsedSeconds :type Float%20%28double-precision%29) (TriggeredSeconds :type Float%20%28double-precision%29) (InputAction :type Input%20Action%20Object%20Reference :default "/Game/Player/Input/Actions/IA_Handbreak.IA_Handbreak"))
  (bind _vehicle_movement_component (Variables|Default|GetVehicle%20Movement%20Component))
  (:Triggered
    (Class|ChaosVehicleMovementComponent|SetHandbrakeInput _vehicle_movement_component true))
  (:Completed
    (Class|ChaosVehicleMovementComponent|SetHandbrakeInput _vehicle_movement_component false)))

(event Input|EnhancedActionEvents|EnhancedInputActionIA_LookAround
  (params (ActionValue :type Float%20%28double-precision%29) (ElapsedSeconds :type Float%20%28double-precision%29) (TriggeredSeconds :type Float%20%28double-precision%29) (InputAction :type Input%20Action%20Object%20Reference :default "/Game/Player/Input/Actions/IA_LookAround.IA_LookAround"))
  (Transformation|AddLocalRotation (Variables|Default|GetSpringArm) (Math|Rotator|MakeRotator 0.0 0.0 ActionValue) false false))

(event Input|EnhancedActionEvents|EnhancedInputActionIA_Exit
  (params (ActionValue :type Boolean) (ElapsedSeconds :type Float%20%28double-precision%29) (TriggeredSeconds :type Float%20%28double-precision%29) (InputAction :type Input%20Action%20Object%20Reference :default "/Game/Player/Input/Actions/IA_Exit.IA_Exit"))
  (bind _returnvalue (Actor|GetActorOfClass "/Game/Player/BP_Player.BP_Player_C"))
  (Transformation|SetActorTransform _returnvalue (Transformation|GetWorldTransform (Variables|Default|GetArrow)) false true)
  (Rendering|SetActorHiddenInGame _returnvalue false)
  (Collision|SetCollisionEnabled (Variables|/Script/Engine.Character|GetCapsuleComponent _returnvalue) "QueryAndPhysics")
  (Collision|SetCollisionEnabled (Variables|/Script/Engine.Character|GetMesh _returnvalue) "QueryOnly")
  (Pawn|Possess (Game|GetPlayerController 0) _returnvalue))

(event EventTick
  (params (DeltaSeconds :type Float%20%28single-precision%29))
  (Class|PrimitiveComponent|SetAngularDamping (Variables|Default|GetVehicleMesh) (Math|Float|SelectFloat 0.0 3.0 (AI|Components|NavMovement|IsMovingonGround (Variables|Default|GetVehicle%20Movement%20Component))))
  (CallFunction|InterpstoOriginalRotation))

(event EventPossessed
  (params (NewController :type Controller%20Object%20Reference))
  (Input|AddMappingContext (PlayerController|LocalPlayerSubsystems|GetEnhancedInputLocalPlayerSubsystem (Game|GetPlayerController 0)) "/Game/Player/Input/IMC_Car.IMC_Car" 0 "(bIgnoreAllPressedKeysUntilRelease=True,bForceImmediately=False,bNotifyUserSettings=False)"))

(event EventUnpossessed
  (params (OldController :type Controller%20Object%20Reference))
  (Input|RemoveMappingContext (PlayerController|LocalPlayerSubsystems|GetEnhancedInputLocalPlayerSubsystem (Game|GetPlayerController 0)) "/Game/Player/Input/IMC_Car.IMC_Car" "(bIgnoreAllPressedKeysUntilRelease=True,bForceImmediately=False,bNotifyUserSettings=False)"))

(fn ConstructionScript)